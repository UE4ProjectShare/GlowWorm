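; Firefly swarm spawner, built on an inherited flocking system, that scatters from an entering actor and follows it when it leaves.
; BeginPlay spawns glow worms within the spawn radius and periodically randomizes their separation.
; Sphere overlap adds threats; exit clears them, retunes flocking and redirects wander targets around that actor.
; A timer hides leader instances and adjusts flock speed by their distance to it, while tracked worms are destroyed after a delay.
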(event `self.ReceiveBeginPlay`
  (bind _spawnradius (`self.SpawnRadius`))
  (`|ExecutionSequence`
    (:`then_0`
      ;[1 1 1] 生成萤火虫
      (for _ (range (+ (`self.NumOfGlowWorms`) 1))
        (`self.AddGlowWormToWorldSpace` (`KismetMathLibrary.MakeTransform` (+ (`self.K2_GetActorLocation`) (* (`KismetMathLibrary.RandomUnitVector`) (`KismetMathLibrary.RandomFloatInRange` 1.0 _spawnradius))) (`KismetMathLibrary.RandomRotator` false) (1.0 1.0 1.0)))))
    (:`then_1`
      ;[1 1 1] 改变萤火虫之间的距离
      (set `self.FlockRadius` _spawnradius)
      (`KismetSystemLibrary.K2_SetTimerDelegate` (delegate `CustomEvent_0`) 2.0 true))))

(event `CustomEvent_0`
  ;[1 1 1] 改变萤火虫之间的距离
  (set `self.SeperationRadius` (`KismetMathLibrary.RandomFloatInRange` 0.0 50.0)))

(event `self.pSphereComponent.OnComponentBeginOverlap`
  (params (OverlappedComponent :type "PrimitiveComponent Object Reference") (OtherActor :type "Actor Object Reference") (OtherComp :type "PrimitiveComponent Object Reference") (OtherBodyIndex :type Integer) (bFromSweep :type Boolean) (SweepResult :type "HitResult Structure (by ref)"))
  ;[1 1 1] 角色走进萤火虫群，会自动散开
  (`KismetArrayLibrary.Array_Add` (`self.Threats`) OtherActor)
  (set `self.FlockMaxSpeed` 100.0))

(event `self.pSphereComponent.OnComponentEndOverlap`
  (params (OverlappedComponent :type "PrimitiveComponent Object Reference") (OtherActor :type "Actor Object Reference") (OtherComp :type "PrimitiveComponent Object Reference") (OtherBodyIndex :type Integer))
  ;[1 1 1] 角色离开萤火虫群体，跟随
  (`|ExecutionSequence`
    (:`then_0`
      (set `self.OtherActor` OtherActor)
      (`KismetArrayLibrary.Array_Clear` (`self.Threats`))
      (set `self.FlockMaxSpeed` 100.0)
      (set `self.ChangeLeaderLocation` true)
      (set `self.FlockMateRotationRate` 5.0)
      (set `self.SeperationRadius` 50.0)
      (set `self.SeperationScale` 20.0)
      (set `self.CohesionScale` 0.3)
      (`KismetSystemLibrary.K2_SetTimerDelegate` (delegate `CustomEvent_1`) 0.1 true))
    (:`then_1`
      (`KismetSystemLibrary.Delay` 10.0)
      (for _array_element (`self.GrowWormInstanceArr`)
        (`self.K2_DestroyActor` _array_element)))))

(event `CustomEvent_1`
  (bind _otheractor (`self.OtherActor`))
  ;[1 1 1] 角色离开萤火虫群体，跟随
  (bind _outactors (`GameplayStatics.GetAllActorsOfClass` "/GlowWorm/BP_GrowWormInstance.BP_GrowWormInstance_C"))
  (for _array_element _outactors
    (if (`GrowWormInstance.IsLeader` _array_element)
      (`self.SetActorHiddenInGame` _array_element true)
      (`/Engine/EditorBlueprintResources/StandardMacros.IsValid` _otheractor
        (:`Is Valid`
          (if (< (`KismetMathLibrary.VSize` (- (`self.K2_GetActorLocation` _array_element) (`self.K2_GetActorLocation` _otheractor))) 220.0)
            (set `self.FlockMaxSpeed` 25.0)
            (else
              (set `self.FlockMaxSpeed` 300.0))))))))

(event `self.ReceiveTick`
  (params (DeltaSeconds :type "Float (single-precision)"))
  ;[1 1 1] 角色离开萤火虫群体，跟随
)

(fn `GetRandomWanderLocation`
  (returns (ReturnValue :type "Vector Structure"))
  (`parent.GetRandomWanderLocation`)
  (if (`self.ChangeLeaderLocation`)
    (return (+ (`self.K2_GetActorLocation` (`self.OtherActor`)) (* (`KismetMathLibrary.RandomUnitVector`) 50.0)))
    (else
      (return (+ (`self.K2_GetActorLocation`) (* (`KismetMathLibrary.RandomUnitVector`) (`self.FlockRadius`)))))))

(fn `UserConstructionScript`
  (`SphereComponent.SetSphereRadius` (`self.pSphereComponent`) (`self.SpawnRadius`) true))